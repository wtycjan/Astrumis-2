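; Player character for Astrumis that manages its input mode, Guitar Hero UI panel and monster-attack death sequence.
; On authority BeginPlay it sets game-only input, creates the hidden panel and binds to the UI subsystem's toggle event.
; Showing the panel switches to UI-only input and freezes the character through CustomTimeDilation.
; A monster attack disables input and movement, snaps view yaw toward the monster and animates pitch with a timeline.
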(event `self.ReceiveBeginPlay`
  (bind _asplayer_controller (cast `PlayerController` (`self.GetController`) :!pure true))
  ;[0.09074 1 0] BeginPlay
  (`/Engine/EditorBlueprintResources/ActorMacros.Switch Has Authority`
    (:`Authority`
      (`parent.ReceiveBeginPlay`)
      (`WidgetBlueprintLibrary.SetInputMode_GameOnly` _asplayer_controller)
      (set `PlayerController.bShowMouseCursor` false _asplayer_controller)
      (`self.CreateUIs`))))

(event `OnAttackedByMonster`
  (params (MonsterLocation :type "Vector Structure"))
  ;[1 1 1] Death
  (set `self.bPlayerInput` false)
  (`ActorComponent.Deactivate` (`self.CharacterMovement`))
  (`Controller.SetControlRotation` (`self.GetController`) (`KismetMathLibrary.MakeRotator` 0.0 10.0 (.yaw (`KismetMathLibrary.FindLookAtRotation` (`self.K2_GetActorLocation`) MonsterLocation))))
  (bind (_direction _delta) (`Timeline|Timeline` :!via `PlayFromStart`)
    (:`Update`
      (`self.AddControllerPitchInput` _delta))))

(event `CreateUIs`
  ;[0 1 0.0832] Create UI Panels
  (`self.CreateGuitarHeroPanel`)
  (add `/Game/Astrumis/Core/BP_UISubsystem.ToggleGuitarHeroWindow` (subsystem `/Game/Astrumis/Core/BP_UISubsystem`) (`|CreateDelegate` :!event `ToggleGuitarHeroPanel`)))

(event `CreateGuitarHeroPanel`
  ;[1 1 1] Guitar Hero
  (bind _returnvalue (`|CreateWidget` "/Game/Astrumis/Minigames/GuitarHero/WBP_GuitarHero_S.WBP_GuitarHero_S_C" (cast `PlayerController` (`self.GetController`) :!pure true)))
  (bind _output_get (set `self.GuitarHeroPanel` _returnvalue))
  (`UserWidget.AddToViewport` _returnvalue 0)
  (`UserWidget.AddToViewport` _output_get 0)
  (`Widget.SetVisibility` _output_get "Hidden"))

(event `ToggleGuitarHeroPanel`
  (params (bVisible :type Boolean))
  ;[1 1 1] Guitar Hero
  (`self.ToggleWindowUI` bVisible (`self.GuitarHeroPanel`)))

(fn `ToggleWindowUI`
  (params (bVisible :type Boolean) (Window :type "Widget Object Reference"))
  (bind _window (`local.Window`))
  (if bVisible
    (`Widget.SetVisibility` _window "Visible")
    (set `self.CustomTimeDilation` 0.0)
    (`WidgetBlueprintLibrary.SetInputMode_UIOnlyEx` (cast `PlayerController` (`self.GetController`) :!pure true) _window)
    (else
      (`Widget.SetVisibility` (`local.Window`) "Hidden")
      (set `self.CustomTimeDilation` 1.0)
      (`WidgetBlueprintLibrary.SetInputMode_GameOnly` (cast `PlayerController` (`self.GetController`) :!pure true)))))

(fn `UserConstructionScript`
  (`parent.UserConstructionScript`))
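; Mission Control player in a two-role game where the host is the Survivor, watching the level through switchable fixed cameras.
; On the client, it builds the HUD, quest log, passwords, guitar-hero minigame and confirmation widgets.
; A timed mouse-cursor trace focuses interactables, pausing while either popup panel is open, and clicks send interactions through server events.
; Camera switches also advance quests, while server events handle level travel and password population.
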(event `self.ReceiveBeginPlay`
  (bind _asplayer_controller (cast `PlayerController` (`self.GetController`) :!pure true))
  ;[0.07654 1 0] BeginPlay
  ;;[1 1 1] TODO #1: Character selection - for now host is always Survivor
  (`/Engine/EditorBlueprintResources/ActorMacros.Switch Has Authority`
    (:`Remote`
      (bind _returnvalue (`GameplayStatics.GetActorOfClass` "/Game/Astrumis/Characters/BP_AstrumisPlayerCharacter.BP_AstrumisPlayerCharacter_C"))
      (set `self.PlayerSurvivor` _returnvalue)
      (bind _returnvalue_2 (`|CreateWidget` "/Game/Astrumis/Core/UI/WBP_MissionControlHUD.WBP_MissionControlHUD_C" _asplayer_controller))
      (`UserWidget.AddToViewport` _returnvalue_2 0)
      (`/Game/Astrumis/Core/UI/WBP_MissionControlHUD.Setup` _returnvalue_2 (`self.PlayerSurvivor`))
      (set `self.CoreHUD` _returnvalue_2)
      (add `/Game/Astrumis/Core/UI/WBP_MissionControlHUD.OnCameraButtonPressed` _returnvalue_2 (delegate `OnCameraButtonPressed`))
      (set `PlayerController.bShowMouseCursor` true _asplayer_controller)
      (`WidgetBlueprintLibrary.SetInputMode_GameAndUIEx` _asplayer_controller null "DoNotLock" false)
      (`PlayerController.SetViewTargetWithBlend` _asplayer_controller (`|GetArrayItem` (`self.Cameras`) (`self.StartingCameraIndex`)) 0.0 "VTBlend_Linear" 0.0 false)
      (`KismetSystemLibrary.K2_SetTimer` null "TraceForInteraction" 0.1 true)
      (`self.CreateUIs`))))

(event `OnCameraButtonPressed`
  (params (CameraIndex :type Integer))
  (bind _returnvalue (subsystem `/Game/Astrumis/Quests/BP_QuestSubsystem`))
  ;[1 1 1] Change Camera
  (`PlayerController.SetViewTargetWithBlend` (cast `/Game/Astrumis/PlayerControllers/BP_AstrumisPlayerController` (`self.GetController`) :!pure true) (`|GetArrayItem` (`self.Cameras`) CameraIndex) 0.0 "VTBlend_Linear" 0.0 false)
  (switch `int` CameraIndex
    (:`0`
      (`QuestSubsystem.TryCompleteQuest` _returnvalue "/Game/Astrumis/Quests/Quests/Tutorial/BP_Quest_MC_T_2.BP_Quest_MC_T_2_C"))
    (:`4`
      (`QuestSubsystem.TryCompleteQuest` _returnvalue "/Game/Astrumis/Quests/Quests/Tutorial/BP_Quest_MC_T_5.BP_Quest_MC_T_5_C")))
  (`self.ChangeCameraOnServer`))

(event `self.ReceiveDestroyed`
  ;[1 1 1] Destroyed
  (`/Game/Astrumis/GameInstances/BP_AstrumisGameInstance.ClearData` (cast `/Game/Astrumis/GameInstances/BP_AstrumisGameInstance` (`GameplayStatics.GetGameInstance`) :!pure true)))

(event `ChangeCameraOnServer`
  (bind _returnvalue (subsystem `/Game/Astrumis/Quests/BP_QuestSubsystem`))
  ;[1 1 1] Change Camera
  (`QuestSubsystem.TryCompleteQuest` _returnvalue "/Game/Astrumis/Quests/Quests/Tutorial/BP_Quest_S_T_2.BP_Quest_S_T_2_C")
  (`QuestSubsystem.TryCompleteQuest` _returnvalue "/Game/Astrumis/Quests/Quests/Tutorial/BP_Quest_S_T_5.BP_Quest_S_T_5_C"))

(event `ServerTravel`
  (params (LevelToLoad :type String))
  ;[0.8803 0.2319 1] ServerTravel
  (`self.ServerTravelOnServer` LevelToLoad))

(event `ServerTravelOnServer`
  (params (LevelToLoad :type String))
  ;[0.8803 0.2319 1] ServerTravel
  (`/Game/Astrumis/GameInstances/BP_AstrumisGameInstance.ClearData` (cast `/Game/Astrumis/GameInstances/BP_AstrumisGameInstance` (`GameplayStatics.GetGameInstance`) :!pure true))
  (bind _asbp_astrumis_player_character (cast `/Game/Astrumis/Characters/BP_AstrumisPlayerCharacter` (`GameplayStatics.GetPlayerCharacter` 0)))
  (`/Game/Astrumis/Characters/BP_AstrumisPlayerCharacter.ServerTravelOnServer` _asbp_astrumis_player_character LevelToLoad))

(event `Key|LeftMouseButton`
  (params (Key :type "Key Structure"))
  ;[1 1 1] Interaction
  (:`Pressed`
    (bind _focusedactor (`self.FocusedActor`)
      (:`then`
        (bind _interaction_component (`/Game/FPFM/Core/Macros/FPFM_MacroLibrary.IsInteractableByPlayer` _focusedactor "MissionControl")
          (:`Is Interactable`
            (`self.ServerInteract` _interaction_component 0 self))))
      (:`else`)))
  (:`Released`
    (bind _focusedactor_2 (`self.FocusedActor`)
      (:`then`
        (bind _interaction_component_2 (`/Game/FPFM/Core/Macros/FPFM_MacroLibrary.IsInteractableByPlayer` _focusedactor_2 "MissionControl")
          (:`Is Interactable`
            (`self.ServerEndInteract` _interaction_component_2))))
      (:`else`))))

(event `ServerInteract`
  (params (InteractionComponent :type "/Game/FPFM/Core/Components/FPFM_InteractionComponent Object Reference") (InteractionIndex :type Integer) (Interactor :type "Actor Object Reference"))
  ;[1 1 1] Interaction
  (`/Game/FPFM/Core/Components/FPFM_InteractionComponent.Interact` InteractionComponent InteractionIndex Interactor))

(event `ServerEndInteract`
  (params (InteractionComponent :type "/Game/Astrumis/Core/BP_InteractableComponent Object Reference"))
  ;[1 1 1] Interaction
  (`/Game/Astrumis/Core/BP_InteractableComponent.EndInteraction` InteractionComponent))

(event `CreateUIs`
  ;[0 1 0.0832] Create UI Panels
  (`self.CreateGuitarHeroPanel`)
  (add `/Game/Astrumis/Core/BP_UISubsystem.ToggleGuitarHeroWindow` (subsystem `/Game/Astrumis/Core/BP_UISubsystem`) (`|CreateDelegate` :!event `ToggleGuitarHeroPanel`))
  (`self.CreateQuestLog`)
  (`self.CreatePasswordsHUD`)
  (`self.CreateConfirmationPanel`)
  (add `/Game/Astrumis/Core/BP_UISubsystem.ToggleConfirmationWindow` (subsystem `/Game/Astrumis/Core/BP_UISubsystem`) (`|CreateDelegate` :!event `ToggleConfirmationPanel`)))

(event `CreateGuitarHeroPanel`
  ;[1 1 1] Guitar Hero
  (bind _returnvalue (`|CreateWidget` "/Game/Astrumis/Minigames/GuitarHero/WBP_GuitarHero_MC.WBP_GuitarHero_MC_C" (cast `PlayerController` (`self.GetController`) :!pure true)))
  (bind _output_get (set `self.GuitarHeroPanel` _returnvalue))
  (`UserWidget.AddToViewport` _output_get 0)
  (`Widget.SetVisibility` _output_get "Hidden")
  (set `/Game/Astrumis/Minigames/GuitarHero/WBP_GuitarHero_MC.MissionControl` self _output_get))

(event `CreateConfirmationPanel`
  ;[1 1 1] ConfirmationPanel
  (bind _returnvalue (`|CreateWidget` "/Game/Astrumis/Core/UI/WBP_ConfirmationPanel.WBP_ConfirmationPanel_C" (cast `PlayerController` (`self.GetController`) :!pure true)))
  (bind _output_get (set `self.ConfirmationPanel` _returnvalue))
  (`UserWidget.AddToViewport` _output_get 0)
  (`Widget.SetVisibility` _output_get "Collapsed"))

(event `CreateQuestLog`
  ;[1 1 1] Quest Log
  (bind _returnvalue (`|CreateWidget` "/Game/Astrumis/Quests/UI/WBP_QuestLogHUD.WBP_QuestLogHUD_C" (cast `PlayerController` (`self.GetController`) :!pure true)))
  (bind _output_get (set `self.QuestLogHUD` _returnvalue))
  (`UserWidget.AddToViewport` _output_get 0))

(event `CreatePasswordsHUD`
  ;[1 1 1] Passwords
  (bind _returnvalue (`|CreateWidget` "/Game/Astrumis/Minigames/Passwords/WBP_MissionControlPaswords.WBP_MissionControlPaswords_C" (cast `PlayerController` (`self.GetController`) :!pure true)))
  (bind _output_get (set `self.PasswordsHUD` _returnvalue))
  (`UserWidget.AddToViewport` _output_get 0)
  (`self.PopulatePasswordsOnServer`))

(event `ToggleGuitarHeroPanel`
  (params (bVisible :type Boolean))
  ;[1 1 1] Guitar Hero
  (`self.ToggleWindowUI` bVisible (`self.GuitarHeroPanel`)))

(event `ToggleConfirmationPanel`
  (params (Title :type String) (ToolTip :type String) (bConfirmationEnabled :type Boolean) (bTooltipVisible :type Boolean) (bVisible :type Boolean))
  (bind _confirmationpanel (`self.ConfirmationPanel`))
  ;[1 1 1] ConfirmationPanel
  (`self.ToggleWindowUI` bVisible _confirmationpanel)
  (if bVisible
    (`/Game/Astrumis/Core/UI/WBP_ConfirmationPanel.Setup` _confirmationpanel Title ToolTip bConfirmationEnabled bTooltipVisible)))

(event `PopulatePasswordsOnServer`
  ;[1 1 1] Passwords
  (`self.PopulatePasswordsMulticast`))

(event `PopulatePasswordsMulticast`
  ;[1 1 1] Passwords
  (bind _returnvalue (`GameplayStatics.GetCurrentLevelName` true))
  (bind _outactors (`GameplayStatics.GetAllActorsOfClass` "/Game/Astrumis/Doodads/BP_PasswordLockedDoors.BP_PasswordLockedDoors_C"))
  (`/Game/Astrumis/Minigames/Passwords/WBP_MissionControlPaswords.PopulatePasswords` (`self.PasswordsHUD`) _outactors (`BlueprintMapLibrary.Map_Find` (`MinigameSettings.RandomPasswordCountPerMapName` (`MinigameSubsystem.Settings` (subsystem `/Game/Astrumis/Minigames/BP_MinigamesSubsystem`))) _returnvalue)))

(event `GuitarHero_Button`
  (params (Color :type "/Game/Astrumis/Minigames/GuitarHero/E_Color Enum" :default "NewEnumerator0"))
  ;[1 1 1] GuitarHero
  (`/Game/Astrumis/Minigames/BP_MinigamesSubsystem.CallButtonPressed` (subsystem `/Game/Astrumis/Minigames/BP_MinigamesSubsystem`) Color))

(fn `ToggleWindowUI`
  (params (bVisible :type Boolean) (Widget :type "Widget Object Reference"))
  (`Widget.SetVisibility` Widget (select `bool` bVisible :`false` "Hidden" :`true` "Visible" :!type "ESlateVisibility Enum"))
  (if (`local.bVisible`)
    (`KismetSystemLibrary.K2_PauseTimer` null "TraceForInteraction")
    (else
      (`KismetSystemLibrary.K2_UnPauseTimer` null "TraceForInteraction"))))

(fn `TraceForInteraction`
  (locals (HitActor :type "Actor Object Reference"))
  (bind (_worldlocation _worlddirection) (`PlayerController.DeprojectMousePositionToWorld` (cast `PlayerController` (`self.GetController`) :!pure true)))
  (bind (_outhit _returnvalue) (`KismetSystemLibrary.LineTraceSingle` _worldlocation (+ _worldlocation (* _worlddirection (`self.MouseTraceLength`))) "TraceTypeQuery1"))
  (if _returnvalue
    (set `local.HitActor` (`.HitActor` (`GameplayStatics.BreakHitResult` _outhit)))
    (`self.FocusedActor`
      (:`then`
        ;[0 0 0] Call the unfocus event and clear Focused Actor when character begins looking at a different actor
        (if (not (== (`self.FocusedActor`) (`local.HitActor`)))
          (bind _focusedactor (`self.FocusedActor`)
            (:`then`
              (`/Game/FPFM/Core/Components/FPFM_InteractionComponent.Unfocus` (`self.GetComponentByClass` _focusedactor "/Game/Astrumis/Core/BP_InteractableComponent.BP_InteractableComponent_C"))
              (set `self.FocusedActor` null)
              ;[0 0 0] Check if the hit actor is interactable
              (`/Game/FPFM/Core/Macros/FPFM_MacroLibrary.IsInteractableByPlayer` (`local.HitActor`) "MissionControl" :!label _label
                (:`Is Interactable`
                  ;[0 0 0] Set new Focused Actor and call the focused event when character looks at a new interactable actor
                  (bind _output_get (set `self.FocusedActor` (`local.HitActor`)))
                  (bind _interaction_component (`/Game/FPFM/Core/Macros/FPFM_MacroLibrary.IsInteractableByPlayer` _output_get "MissionControl")
                    (:`Is Interactable`
                      (`/Game/FPFM/Core/Components/FPFM_InteractionComponent.Focus` _interaction_component))))))
            (:`else`))))
      (:`else`
        (goto _label)))
    (else
      ;[0 0 0] Call the unfocus event and clear Focused Actor when trace does not hit any actors
      (bind _focusedactor_2 (`self.FocusedActor`)
        (:`then`
          (bind _interaction_component_2 (`/Game/FPFM/Core/Macros/FPFM_MacroLibrary.IsInteractableByPlayer` _focusedactor_2 "MissionControl")
            (:`Is Interactable`
              (`/Game/FPFM/Core/Components/FPFM_InteractionComponent.Unfocus` _interaction_component_2)
              (set `self.FocusedActor` null))))
        (:`else`)))))

(fn `UserConstructionScript`)
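; BP_Monster is an enemy character that chases the player once it spots them.
; PawnSensing filters seen pawns to BP_AstrumisPlayerCharacter, sets SeePlayer and calls FollowPlayer, which issues AIMoveTo toward that pawn.
; On the authority, Tick stops movement immediately every frame while SeePlayer is false.
; Nothing in the graph clears SeePlayer, so that hold ends after the first sighting.
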(event `self.ReceiveTick`
  (params (DeltaSeconds :type "Float (single-precision)"))
  (`/Engine/EditorBlueprintResources/ActorMacros.Switch Has Authority`
    (:`Authority`
      (if (not (`self.bSeePlayer`))
        (`MovementComponent.StopMovementImmediately` (`self.CharacterMovement`))))))

(event `self.PawnSensing.OnSeePawn`
  (params (Pawn :type "Pawn Object Reference"))
  (cast `/Game/Astrumis/Characters/BP_AstrumisPlayerCharacter` Pawn)
  (set `self.bSeePlayer` true)
  (`self.FollowPlayer`))

(event `FollowPlayer`
  (if (`self.bSeePlayer`)
    (`|AIMoveTo` self (0.0 0.0 0.0) (stale `self.PawnSensing.OnSeePawn` Pawn))))

(fn `UserConstructionScript`)
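; BP_ActionOnEnter is a trigger actor that runs configurable actions when a BP_AstrumisPlayerCharacter begins overlapping it.
; It can play a sound at its location, play dialogue through the subtitles subsystem, and try to complete listed quests.
; If a level is set, it calls ServerTravel on player character 0, not necessarily the overlapping one.
; It can then destroy itself if flagged.
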(event `self.ReceiveActorBeginOverlap`
  (params (OtherActor :type "Actor Object Reference"))
  (bind _soundcue (`self.SoundCue`))
  (bind _leveltoload (`self.LevelToLoad`))
  (bind _dialoguecue (`self.DialogueCue`))
  (cast `/Game/Astrumis/Characters/BP_AstrumisPlayerCharacter` OtherActor)
  (`/Engine/EditorBlueprintResources/StandardMacros.IsValid` _soundcue
    (:`Is Valid`
      (`GameplayStatics.PlaySoundAtLocation` _soundcue (`self.K2_GetActorLocation`) (struct) 1.0 1.0 0.0 null null null null))
    (:`Is Not Valid`
      _))
  (`/Engine/EditorBlueprintResources/StandardMacros.IsValid` _dialoguecue
    (:`Is Valid`
      (`SubtitlesSubsystem.PlayDialogue` (subsystem `/Game/Astrumis/Subtitles/BP_SubtitlesSubsystem`) _dialoguecue (`GameplayStatics.GetPlayerController` 0)))
    (:`Is Not Valid`
      _))
  (for _array_element (`self.QuestsToComplete`)
    (`QuestSubsystem.TryCompleteQuest` (subsystem `/Game/Astrumis/Quests/BP_QuestSubsystem`) _array_element))
  (if (not (`KismetStringLibrary.IsEmpty` _leveltoload))
    (bind _asbp_astrumis_player_character (cast `/Game/Astrumis/Characters/BP_AstrumisPlayerCharacter` (`GameplayStatics.GetPlayerCharacter` 0)))
    (`/Game/Astrumis/Characters/BP_AstrumisPlayerCharacter.ServerTravel` _asbp_astrumis_player_character _leveltoload))
  (if (`self.bDestroy`)
    (`self.K2_DestroyActor`)))

(fn `UserConstructionScript`)
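; Cinematic door actor that opens, closes or gets destroyed, with matching sound.
; One timeline, played or reversed at a rate set by open/close duration, lerps the mesh between opened and closed transforms and tracks state.
; PlaySound starts the cue at an offset derived from the last closing progress.
; Destroy runs a separate timeline from closed to destroyed transform, activating particles and playing a one-shot fall sound near the end.
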(event `Destroy`
  (bind _audio (`self.Audio`))
  ;[1 1 1] Destroy Door
  (`TimelineComponent.SetPlayRate` (`self.DestroyTimeline`) (/ 1.0 (`self.TimeToDestroy`)))
  (`AudioComponent.Stop` _audio)
  (`AudioComponent.SetSound` _audio "/Game/Astrumis/Sounds/Tutorial/Tutorial_OpenDoor_Cue.Tutorial_OpenDoor_Cue")
  (`AudioComponent.Play` _audio 0.0)
  (`ActorComponent.Activate` (`self.ParticleSystem`) true)
  (bind (_direction _newtrack_0) (`Timeline|DestroyTimeline` :!via `PlayFromStart`)
    (:`Update`
      (`SceneComponent.K2_SetRelativeTransform` (`self.DoorMesh`) (`KismetMathLibrary.TLerp` (`self.ClosedTransform`) (`self.DestroyedTransform`) _newtrack_0) false false)
      (if (> _newtrack_0 0.7)
        (`/Engine/EditorBlueprintResources/StandardMacros.DoOnce` false
          (:`Completed`
            (`GameplayStatics.PlaySoundAtLocation` "/Game/Astrumis/Sounds/Tutorial/Tutorial_DoorFallDown_Cue.Tutorial_DoorFallDown_Cue" (`self.K2_GetActorLocation`) (struct) 1.0 1.0 0.0 null null null null)))))))

(event `CloseDoor`
  ;[1 1 1] Open / Close Door
  (set `self.State` "NewEnumerator3")
  (`self.PlaySound`)
  (`TimelineComponent.SetPlayRate` (`self.DoorTimeline`) (/ 1.0 (`self.TimeToClose`)))
  (bind (_direction _doorrotate) (`Timeline|DoorTimeline` :!label _label)
    (:`Update`
      (bind _output_get (set `self.ClosingDelta` _doorrotate))
      (`SceneComponent.K2_SetRelativeTransform` (`self.DoorMesh`) (`KismetMathLibrary.TLerp` (`self.OpenedTransform`) (`self.ClosedTransform`) _output_get) false false))
    (:`Finished`
      (switch `/Game/Astrumis/Doodads/E_DoorState` (`self.State`)
        (:`NewEnumerator2`
          (set `self.State` "NewEnumerator1"))
        (:`NewEnumerator3`
          (set `self.State` "NewEnumerator0"))))))

(event `OpenDoor`
  ;[1 1 1] Open / Close Door
  (set `self.State` "NewEnumerator2")
  (`self.PlaySound`)
  (`TimelineComponent.SetPlayRate` (`self.DoorTimeline`) (/ 1.0 (`self.TimeToOpen`)))
  (goto _label :!via `ReverseFromEnd`))

(fn `PlaySound`
  (locals (DelayTime :type "Float (double-precision)") (Sound :type "SoundBase Object Reference"))
  (bind _audio (`self.Audio`))
  (`|ExecutionSequence`
    (:`then_0`
      (switch `/Game/Astrumis/Doodads/E_DoorState` (`self.State`)
        (:`NewEnumerator2`
          (set `local.DelayTime` (* (`KismetMathLibrary.Abs` (- (`self.ClosingDelta`) 1.0)) (`self.TimeToOpen`)))
          (set `local.Sound` "/Game/Astrumis/Sounds/Interactions/CUE_DoorOpen.CUE_DoorOpen"))
        (:`NewEnumerator3`
          (set `local.DelayTime` (* (`self.ClosingDelta`) (`self.TimeToClose`)))
          (set `local.Sound` "/Game/Astrumis/Sounds/Interactions/CUE_DoorClose.CUE_DoorClose"))))
    (:`then_1`
      (`AudioComponent.Stop` _audio)
      (`AudioComponent.SetSound` _audio (`local.Sound`))
      (`AudioComponent.Play` _audio (`local.DelayTime`)))))

(fn `UserConstructionScript`
  (`parent.UserConstructionScript`))
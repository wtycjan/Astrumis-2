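; Double sliding door doodad that opens and closes when clicked or interacted with through its interactable component.
; A DoOnce gate guards each toggle until the timeline finishes, with play rate derived from the open or close time.
; The timeline slides two meshes in mirrored directions, and the IsOpen RepNotify snaps them to the matching end position.
; A glow shows on cursor hover when the door is interactable by the MissionControl player type.
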(event `self.ReceiveBeginPlay`
  ;[0.1218 1 0] BeginPlay
  (add `self.OnClicked` (delegate `OnClicked_Event`)))

(event `OnClicked_Event` :!signature `self.OnClicked`
  (params (TouchedActor :type "Actor Object Reference") (ButtonPressed :type "Key Structure" :default "None"))
  ;[0.1218 1 0] BeginPlay
  (`/Game/Astrumis/Core/BP_InteractableComponent.Click` (`self.BP_InteractableComponent`)))

(event `self.BP_InteractableComponent.OnInteract`
  (params (InteractionIndex :type Integer) (Interactor :type "Actor Object Reference"))
  (`/Engine/EditorBlueprintResources/StandardMacros.DoOnce` false :!label _label
    (:`Completed`
      (if (`self.IsOpen?`)
        (`self.CloseDoor`)
        (`KismetSystemLibrary.Delay` (`self.TimeToOpen`))
        (set `self.IsOpen?` false)
        (else
          (`self.OpenDoor`)
          (`KismetSystemLibrary.Delay` (`self.TimeToOpen`))
          (set `self.IsOpen?` true))))))

(event `ResetDoOnce`
  (goto _label :!via `Reset`))

(event `OpenDoor`
  (`TimelineComponent.SetPlayRate` (`self.DoorTimeline`) (/ 1.0 (`self.TimeToOpen`)))
  (bind (_direction _doorrotate) (`Timeline|DoorTimeline` :!via `PlayFromStart` :!label _label_2)
    (:`Update`
      (`SceneComponent.K2_SetRelativeLocation` (`self.DoorMeshA`) (`KismetMathLibrary.VLerp` (`self.ClosePosition`) (`self.OpenPosition`) _doorrotate) false false)
      (`SceneComponent.K2_SetRelativeLocation` (`self.DoorMeshB`) (`KismetMathLibrary.VLerp` (* (`self.ClosePosition`) -1.0) (* (`self.OpenPosition`) -1.0) _doorrotate) false false))
    (:`Finished`
      (`self.ResetDoOnce`))))

(event `CloseDoor`
  (`TimelineComponent.SetPlayRate` (`self.DoorTimeline`) (/ 1.0 (`self.TimeToClose`)))
  (goto _label_2 :!via `ReverseFromEnd`))

(event `self.Glow.OnBeginCursorOver`
  (params (TouchedComponent :type "PrimitiveComponent Object Reference"))
  (`/Game/FPFM/Core/Macros/FPFM_MacroLibrary.IsInteractableByPlayer` self "MissionControl"
    (:`Is Interactable`
      (`SceneComponent.SetVisibility` (`self.Glow`) true false))))

(event `self.Glow.OnEndCursorOver`
  (params (TouchedComponent :type "PrimitiveComponent Object Reference"))
  (`/Game/FPFM/Core/Macros/FPFM_MacroLibrary.IsInteractableByPlayer` self "MissionControl"
    (:`Is Interactable`
      (`SceneComponent.SetVisibility` (`self.Glow`) false false))))

(fn `OnRep_IsOpen?`
  (`SceneComponent.K2_SetRelativeLocation` (`self.DoorMeshA`) (`KismetMathLibrary.SelectVector` (`self.OpenPosition`) (`self.ClosePosition`) (`self.IsOpen?`)) false false)
  (`SceneComponent.K2_SetRelativeLocation` (`self.DoorMeshB`) (`KismetMathLibrary.SelectVector` (* (`self.OpenPosition`) -1.0) (* (`self.ClosePosition`) -1.0) (`self.IsOpen?`)) false false))

(fn `UserConstructionScript`
  (`parent.UserConstructionScript`))
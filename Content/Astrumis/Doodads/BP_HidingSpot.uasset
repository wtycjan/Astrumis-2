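; BP_HidingSpot is a trigger volume that marks the player as hidden while they are inside its box.
; Overlap begin and end toggle the HidingSpot flag on the player character.
; If the monster cached at BeginPlay is at least 1000 units away on entry, the spot clears the monster's bPlayerDetected blackboard key and resets an entry in its AI controller's PreviousSenses array.
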(event `self.ReceiveBeginPlay`
  (bind _returnvalue (`GameplayStatics.GetActorOfClass` "/Game/Astrumis/Characters/BP_Monster.BP_Monster_C"))
  (set `self.Monster` _returnvalue))

(event `self.Box.OnComponentBeginOverlap`
  (params (OverlappedComponent :type "PrimitiveComponent Object Reference") (OtherActor :type "Actor Object Reference") (OtherComp :type "PrimitiveComponent Object Reference") (OtherBodyIndex :type Integer) (bFromSweep :type Boolean) (SweepResult :type "HitResult Structure (by ref)"))
  (bind _monster (`self.Monster`))
  (bind _asbp_astrumis_player_character (cast `/Game/Astrumis/Characters/BP_AstrumisPlayerCharacter` OtherActor))
  (set `/Game/Astrumis/Characters/BP_AstrumisPlayerCharacter.bHidingSpot` true _asbp_astrumis_player_character)
  (if (not (< (`KismetMathLibrary.Vector_Distance` (`self.K2_GetActorLocation` _monster) (`self.K2_GetActorLocation` _asbp_astrumis_player_character)) 1000.0))
    (bind _asaic_monster (cast `/Game/Astrumis/AI/AIC_Monster` (`AIBlueprintHelperLibrary.GetAIController` _monster)))
    (`BlackboardComponent.SetValueAsBool` (`AIBlueprintHelperLibrary.GetBlackboard` _asaic_monster) "bPlayerDetected" false)
    (`KismetArrayLibrary.Array_Set` (`/Game/Astrumis/AI/AIC_Monster.PreviousSenses` _asaic_monster))))

(event `self.Box.OnComponentEndOverlap`
  (params (OverlappedComponent :type "PrimitiveComponent Object Reference") (OtherActor :type "Actor Object Reference") (OtherComp :type "PrimitiveComponent Object Reference") (OtherBodyIndex :type Integer))
  (bind _asbp_astrumis_player_character (cast `/Game/Astrumis/Characters/BP_AstrumisPlayerCharacter` OtherActor))
  (set `/Game/Astrumis/Characters/BP_AstrumisPlayerCharacter.bHidingSpot` false _asbp_astrumis_player_character))

(fn `UserConstructionScript`)
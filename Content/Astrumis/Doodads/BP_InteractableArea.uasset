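; BP_InteractableArea is a placeable interaction point that completes quests when the player interacts with it.
; On BeginPlay it copies its InteractionText into the interactable component's tooltip.
; Interacting runs CompleteQuests, which passes each entry in QuestsToComplete to the quest subsystem's TryCompleteQuest.
; When SingleUse is set, the actor destroys itself after a short delay.
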(event `self.ReceiveBeginPlay`
  ;[0.05442 1 0] BeginPlay
  (set `/Game/FPFM/Core/Components/FPFM_InteractionComponent.TooltipText` (`self.InteractionText`) (`self.BP_InteractableComponent`)))

(event `self.BP_InteractableComponent.OnInteract`
  (params (InteractionIndex :type Integer) (Interactor :type "Actor Object Reference"))
  ;[1 1 1] Interact / End Interact
  (`self.CompleteQuests`))

(event `CompleteQuests`
  ;[1 1 1] CompleteQuests
  (for _array_element (`self.QuestsToComplete`)
    (`QuestSubsystem.TryCompleteQuest` (subsystem `/Game/Astrumis/Quests/BP_QuestSubsystem`) _array_element))
  (if (`self.bSingleUse`)
    (`KismetSystemLibrary.Delay` 0.1)
    (`self.K2_DestroyActor`)))

(fn `UserConstructionScript`)
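; Cockpit interactable area that the player uses to try to take control of the ship.
; Interaction from its interactable component runs a check on the keycard component's locked state.
; While locked, it asks the quest subsystem to try completing two quests; when unlocked, it loads the main menu level.
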(event `self.BP_InteractableComponent.OnInteract`
  (params (InteractionIndex :type Integer) (Interactor :type "Actor Object Reference"))
  ;[1 1 1] Interact / End Interact
  (`self.TryControlShip`))

(event `TryControlShip`
  (bind _returnvalue (subsystem `QuestSubsystem`))
  (if (`/Game/Astrumis/Doodads/BP_KeycardComponent.bLocked` (`self.BP_KeycardComponent`))
    (`QuestSubsystem.TryCompleteQuest` _returnvalue "/Game/Astrumis/Quests/Quests/ShipInterior/BP_Quest_S_SI_1.BP_Quest_S_SI_1_C")
    (`QuestSubsystem.TryCompleteQuest` _returnvalue "/Game/Astrumis/Quests/Quests/ShipInterior/BP_Quest_MC_SI_1.BP_Quest_MC_SI_1_C")
    (else
      (`GameplayStatics.OpenLevel` "MainMenu"))))

(fn `UserConstructionScript`
  (`parent.UserConstructionScript`))
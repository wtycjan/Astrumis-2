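; BP_Keycard is an interactable pickup actor that unlocks the actors tied to it.
; On interact, it loops through ActorsRequiringKeycard and toggles the locked status on each one's BP_KeycardComponent, then destroys itself.
; The interaction also plays a keycard-found voice cue at the keycard's location.
; Because it toggles rather than sets the lock, targets that start unlocked become locked.
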(event `self.BP_InteractableComponent.OnInteract`
  (params (InteractionIndex :type Integer) (Interactor :type "Actor Object Reference"))
  ;[1 1 1] Interact / End Interact
  (`self.UnlockKeycard` Interactor)
  (`GameplayStatics.PlaySoundAtLocation` "/Game/Astrumis/Sounds/Voices/ConstructingMap/CUE_Voice_Snake_KeycardFound.CUE_Voice_Snake_KeycardFound" (`self.K2_GetActorLocation`) (struct) 1.0 1.0 0.0 null null null null))

(event `UnlockKeycard`
  (params (Interactor :type "Actor Object Reference"))
  ;[1 1 1] Open / Close Door
  (for _array_element (`self.ActorsRequiringKeycard`)
    (`/Game/Astrumis/Doodads/BP_KeycardComponent.ToggleLockedStatus` (`self.GetComponentByClass` _array_element "/Game/Astrumis/Doodads/BP_KeycardComponent.BP_KeycardComponent_C")))
  (`self.K2_DestroyActor`))

(fn `UserConstructionScript`
  (`parent.UserConstructionScript`))
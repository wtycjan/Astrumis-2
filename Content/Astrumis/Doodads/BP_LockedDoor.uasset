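; BP_LockedDoor is a keycard-gated door that returns the game to the MainMenu level when opened.
; Its interactable component plays a "keycard needed" voice line at the door while the keycard component is locked, and otherwise triggers OpenLockedDoor, which loads the menu.
; When the keycard component unlocks, the interaction tooltip changes to an open-door prompt.
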(event `self.BP_InteractableComponent.OnInteract`
  (params (InteractionIndex :type Integer) (Interactor :type "Actor Object Reference"))
  ;[1 1 1] Interact / End Interact
  (if (`/Game/Astrumis/Doodads/BP_KeycardComponent.bLocked` (`self.BP_KeycardComponent`))
    (`GameplayStatics.PlaySoundAtLocation` "/Game/Astrumis/Sounds/Voices/ConstructingMap/CUE_Voice_Snake_KeycardNeeded.CUE_Voice_Snake_KeycardNeeded" (`self.K2_GetActorLocation`) (struct) 1.0 1.0 0.0 null null null null)
    (else
      (`self.OpenLockedDoor` null))))

(event `OpenLockedDoor`
  (params (Interactor :type "Actor Object Reference"))
  ;[1 1 1] Open Locked Door
  (`GameplayStatics.OpenLevel` "MainMenu"))

(event `self.BP_KeycardComponent.Unlock`
  (set `/Game/FPFM/Core/Components/FPFM_InteractionComponent.TooltipText` "Press (F) to open door." (`self.BP_InteractableComponent`)))

(fn `UserConstructionScript`
  (`parent.UserConstructionScript`))
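; Interactable lockpicking panel that lets players override a lock through a labyrinth minigame.
; Interacting starts the minigame component, if active, and shows the multiplayer labyrinth window with a randomly picked maze.
; Success disables the box's collision and further interaction.
; Failure lights an alarm and deactivates the minigame for a short cooldown, updating the tooltip until it resets.
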(event `self.BP_InteractableComponent.OnInteract`
  (params (InteractionIndex :type Integer) (Interactor :type "Actor Object Reference"))
  ;[1 1 1] Interact / End Interact
  (if (`ActorComponent.IsActive` (`self.BP_MinigameComponent`))
    (`self.StartLockpicking` Interactor)))

(event `StartLockpicking`
  (params (Interactor :type "Actor Object Reference"))
  ;[1 1 1] Open / Close Door
  (`/Game/Astrumis/Minigames/BP_MinigameComponent.StartMinigame` (`self.BP_MinigameComponent`) Interactor)
  (`/Game/Astrumis/Core/BP_UISubsystem.ToggleMultiplayerLabyrinthWindow` (subsystem `/Game/Astrumis/Core/BP_UISubsystem`) true (`.OutIndex` (`KismetArrayLibrary.Array_Random` (`MinigameSettings.PointCoordinatesPerMaze` (`MinigameSubsystem.Settings` (subsystem `/Game/Astrumis/Minigames/BP_MinigamesSubsystem`)))))))

(event `self.BP_MinigameComponent.OnSuccess`
  ;[1 1 1] Minigame
  (`PrimitiveComponent.SetCollisionEnabled` (`self.Box`) "NoCollision")
  (set `/Game/FPFM/Core/Components/FPFM_InteractionComponent.InteractingPlayerType` "None" (`self.BP_InteractableComponent`)))

(event `self.BP_MinigameComponent.OnFail`
  ;[1 1 1] Minigame
  (`SceneComponent.SetVisibility` (`self.PointLight`) true false)
  (`ActorComponent.Deactivate` (`self.BP_MinigameComponent`))
  (set `/Game/FPFM/Core/Components/FPFM_InteractionComponent.TooltipText` "Alarm triggered! Try again later." (`self.BP_InteractableComponent`))
  (`KismetSystemLibrary.Delay` 4.0)
  (`ActorComponent.Activate` (`self.BP_MinigameComponent`) false)
  (set `/Game/FPFM/Core/Components/FPFM_InteractionComponent.TooltipText` "Press (F) to override lock." (`self.BP_InteractableComponent`))
  (`SceneComponent.SetVisibility` (`self.PointLight`) false false))

(fn `UserConstructionScript`
  (`parent.UserConstructionScript`))
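; BP_NoiseGenerator is an interactable doodad that makes a noise when used.
; Interacting through BP_InteractableComponent calls GenerateNoise, which plays the Audio component and reports a "Noise"-tagged noise event at the actor's location, with itself as instigator.
; The component's focus and unfocus events show and hide a Glow component as a highlight.
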(event `self.BP_InteractableComponent.OnInteract`
  (params (InteractionIndex :type Integer) (Interactor :type "Actor Object Reference"))
  ;[1 1 1] Interact
  (`self.GenerateNoise`))

(event `GenerateNoise`
  ;[1 1 1] Interact
  (`AudioComponent.Play` (`self.Audio`) 0.0)
  (`AISense_Hearing.ReportNoiseEvent` (`self.K2_GetActorLocation`) 1.0 self 0.0 "Noise"))

(event `self.BP_InteractableComponent.OnFocus`
  ;[1 1 1] Focus / UnFocus
  (`SceneComponent.SetVisibility` (`self.Glow`) true false))

(event `self.BP_InteractableComponent.OnUnfocus`
  ;[1 1 1] Focus / UnFocus
  (`SceneComponent.SetVisibility` (`self.Glow`) false false))

(fn `UserConstructionScript`)
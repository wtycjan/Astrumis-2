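; Door that players unlock by entering a password, which makes it slide open.
; Interacting shows the password window and binds to the guitar-hero subsystem's attempt event; a match toggles the password component's lock.
; Unlocking disables further interaction, opens the door and hides player 0's window.
; A rate-scaled timeline lerps the mesh between open and closed positions, with sound start offsets derived from its progress.
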(event `self.BP_InteractableComponent.OnInteract`
  (params (InteractionIndex :type Integer) (Interactor :type "Actor Object Reference"))
  ;[1 1 1] Interact / End Interact
  (bind _asbp_astrumis_player_character (cast `/Game/Astrumis/Characters/BP_AstrumisPlayerCharacter` Interactor))
  (`/Game/Astrumis/Characters/BP_AstrumisPlayerCharacter.TogglePasswordsWindow` _asbp_astrumis_player_character true)
  (add `/Game/Astrumis/Minigames/GuitarHero/BP_GuitarHeroSubsystem.OnAttempt` (subsystem `/Game/Astrumis/Minigames/GuitarHero/BP_GuitarHeroSubsystem`) (delegate `AttemptUnlock`)))

(event `AttemptUnlock`
  (params (EnteredPassword :type String))
  ;[1 1 1] Attempt
  (if (`KismetStringLibrary.EqualEqual_StrStr` EnteredPassword (`/Game/Astrumis/Minigames/Passwords/BP_PasswordComponent.Password` (`self.BP_PasswordComponent`)))
    (`/Game/Astrumis/Minigames/Passwords/BP_PasswordComponent.ToggleLockedStatus` (`self.BP_PasswordComponent`))))

(event `CloseDoor`
  ;[1 1 1] Open / Close Door
  (set `self.State` "NewEnumerator3")
  (`self.PlaySound`)
  (`TimelineComponent.SetPlayRate` (`self.DoorTimeline`) (/ 1.0 (`self.TimeToClose`)))
  (bind (_direction _doorrotate) (`Timeline|DoorTimeline` :!label _label)
    (:`Update`
      (bind _output_get (set `self.ClosingDelta` _doorrotate))
      (`SceneComponent.K2_SetRelativeLocation` (`self.DoorMesh`) (`KismetMathLibrary.VLerp` (`self.OpenPosition`) (`self.ClosePosition`) _output_get) false false))
    (:`Finished`
      (switch `/Game/Astrumis/Doodads/E_DoorState` (`self.State`)
        (:`NewEnumerator2`
          (set `self.State` "NewEnumerator1"))
        (:`NewEnumerator3`
          (set `self.State` "NewEnumerator0"))))))

(event `OpenDoor`
  ;[1 1 1] Open / Close Door
  (set `self.State` "NewEnumerator2")
  (`self.PlaySound`)
  (`TimelineComponent.SetPlayRate` (`self.DoorTimeline`) (/ 1.0 (`self.TimeToOpen`)))
  (goto _label :!via `ReverseFromEnd`))

(event `self.BP_PasswordComponent.Unlock`
  ;[1 1 1] Unlock
  (`self.UnlockOnServer`))

(event `UnlockOnServer`
  ;[1 1 1] Unlock
  (set `/Game/FPFM/Core/Components/FPFM_InteractionComponent.InteractingPlayerType` "None" (`self.BP_InteractableComponent`))
  (`self.OpenDoor`)
  (bind _asbp_astrumis_player_character (cast `/Game/Astrumis/Characters/BP_AstrumisPlayerCharacter` (`GameplayStatics.GetPlayerCharacter` 0)))
  (`/Game/Astrumis/Characters/BP_AstrumisPlayerCharacter.TogglePasswordsWindow` _asbp_astrumis_player_character false))

(fn `PlaySound`
  (locals (DelayTime :type "Float (double-precision)") (Sound :type "SoundBase Object Reference"))
  (bind _audio (`self.Audio`))
  (`|ExecutionSequence`
    (:`then_0`
      (switch `/Game/Astrumis/Doodads/E_DoorState` (`self.State`)
        (:`NewEnumerator2`
          (set `local.DelayTime` (* (`KismetMathLibrary.Abs` (- (`self.ClosingDelta`) 1.0)) (`self.TimeToOpen`)))
          (set `local.Sound` "/Game/Astrumis/Sounds/Interactions/CUE_DoorOpen.CUE_DoorOpen"))
        (:`NewEnumerator3`
          (set `local.DelayTime` (* (`self.ClosingDelta`) (`self.TimeToClose`)))
          (set `local.Sound` "/Game/Astrumis/Sounds/Interactions/CUE_DoorClose.CUE_DoorClose"))))
    (:`then_1`
      (`AudioComponent.Stop` _audio)
      (`AudioComponent.SetSound` _audio (`local.Sound`))
      (`AudioComponent.Play` _audio (`local.DelayTime`)))))

(fn `UserConstructionScript`
  (`parent.UserConstructionScript`))
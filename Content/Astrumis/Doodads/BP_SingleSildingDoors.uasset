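; Single sliding door doodad that opens and closes through its interactable component's interact and end-interact events.
; One timeline, played or reversed at a rate set by open or close time, lerps the mesh between closed and open positions while tracking door state.
; Focus toggles a glow.
; Unfocusing an open or opening door makes the MissionControl pawn send a server end-interact, if that player type can interact with it.
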(event `self.BP_InteractableComponent.OnInteract`
  (params (InteractionIndex :type Integer) (Interactor :type "Actor Object Reference"))
  ;[1 1 1] Interact / End Interact
  (`self.OpenDoor`))

(event `self.BP_InteractableComponent.OnEndInteract`
  ;[1 1 1] Interact / End Interact
  (`self.CloseDoor`))

(event `OpenDoor`
  (set `self.State` "NewEnumerator2")
  (`TimelineComponent.SetPlayRate` (`self.DoorTimeline`) (/ 1.0 (`self.TimeToOpen`)))
  (bind (_direction _doorrotate) (`Timeline|DoorTimeline` :!label _label)
    (:`Update`
      (`SceneComponent.K2_SetRelativeLocation` (`self.DoorMeshA`) (`KismetMathLibrary.VLerp` (`self.ClosePosition`) (`self.OpenPosition`) _doorrotate) false false))
    (:`Finished`
      (switch `/Game/Astrumis/Doodads/E_DoorState` (`self.State`)
        (:`NewEnumerator2`
          (set `self.State` "NewEnumerator1"))
        (:`NewEnumerator3`
          (set `self.State` "NewEnumerator0"))))))

(event `CloseDoor`
  (set `self.State` "NewEnumerator3")
  (`TimelineComponent.SetPlayRate` (`self.DoorTimeline`) (/ 1.0 (`self.TimeToClose`)))
  (goto _label :!via `Reverse`))

(event `self.BP_InteractableComponent.OnFocus`
  ;[1 1 1] Focus / UnFocus
  (`SceneComponent.SetVisibility` (`self.Glow`) true false))

(event `self.BP_InteractableComponent.OnUnfocus`
  ;[1 1 1] Focus / UnFocus
  (`SceneComponent.SetVisibility` (`self.Glow`) false false)
  (switch `/Game/Astrumis/Doodads/E_DoorState` (`self.State`)
    (:`NewEnumerator1`
      _)
    (:`NewEnumerator2`
      _))
  (bind _interaction_component (`/Game/FPFM/Core/Macros/FPFM_MacroLibrary.IsInteractableByPlayer` self "MissionControl")
    (:`Is Interactable`
      (bind _asbp_mission_control (cast `/Game/Astrumis/Characters/BP_MissionControl` (`Controller.K2_GetPawn` (`GameplayStatics.GetPlayerController` 0))))
      (`/Game/Astrumis/Characters/BP_MissionControl.ServerEndInteract` _asbp_mission_control _interaction_component))))

(fn `UserConstructionScript`
  (`parent.UserConstructionScript`))
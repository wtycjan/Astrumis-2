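; Small single sliding door that closes when interacted with and reopens when the interaction ends.
; One timeline, rate-scaled by open and close times, plays or reverses to lerp the mesh between positions while tracking door state.
; PlaySound starts audio at an offset matching door progress, alongside one-shot location sounds.
; Focus shows a glow; unfocusing a closed or closing door makes the MissionControl pawn end the interaction, if interactable by that player type.
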(event `self.BP_InteractableComponent.OnInteract`
  (params (InteractionIndex :type Integer) (Interactor :type "Actor Object Reference"))
  ;[1 1 1] Interact / End Interact
  (`self.CloseDoor`)
  (`GameplayStatics.PlaySoundAtLocation` "/Game/Astrumis/Sounds/Interactions/CUE_DoorClose.CUE_DoorClose" (`self.K2_GetActorLocation`) (struct) 1.0 1.0 0.0 null null null null))

(event `self.BP_InteractableComponent.OnEndInteract`
  ;[1 1 1] Interact / End Interact
  (`self.OpenDoor`)
  (`GameplayStatics.PlaySoundAtLocation` "/Game/Astrumis/Sounds/Interactions/CUE_DoorOpen.CUE_DoorOpen" (`self.K2_GetActorLocation`) (struct) 1.0 1.0 0.0 null null null null))

(event `CloseDoor`
  ;[1 1 1] Open / Close Door
  (set `self.State` "NewEnumerator3")
  (`self.PlaySound`)
  (`TimelineComponent.SetPlayRate` (`self.DoorTimeline`) (/ 1.0 (`self.TimeToClose`)))
  (bind (_direction _doorrotate) (`Timeline|DoorTimeline` :!label _label)
    (:`Update`
      (bind _output_get (set `self.ClosingDelta` _doorrotate))
      (`SceneComponent.K2_SetRelativeLocation` (`self.DoorMesh`) (`KismetMathLibrary.VLerp` (`self.OpenPosition`) (`self.ClosePosition`) _output_get) false false))
    (:`Finished`
      (switch `/Game/Astrumis/Doodads/E_DoorState` (`self.State`)
        (:`NewEnumerator2`
          (set `self.State` "NewEnumerator1"))
        (:`NewEnumerator3`
          (set `self.State` "NewEnumerator0"))))))

(event `OpenDoor`
  ;[1 1 1] Open / Close Door
  (set `self.State` "NewEnumerator2")
  (`self.PlaySound`)
  (`TimelineComponent.SetPlayRate` (`self.DoorTimeline`) (/ 1.0 (`self.TimeToOpen`)))
  (goto _label :!via `Reverse`))

(event `self.BP_InteractableComponent.OnFocus`
  ;[1 1 1] Focus / UnFocus
  (`SceneComponent.SetVisibility` (`self.Glow`) true false))

(event `self.BP_InteractableComponent.OnUnfocus`
  ;[1 1 1] Focus / UnFocus
  (`SceneComponent.SetVisibility` (`self.Glow`) false false)
  (switch `/Game/Astrumis/Doodads/E_DoorState` (`self.State`)
    (:`NewEnumerator0`
      _)
    (:`NewEnumerator3`
      _))
  (bind _interaction_component (`/Game/FPFM/Core/Macros/FPFM_MacroLibrary.IsInteractableByPlayer` self "MissionControl")
    (:`Is Interactable`
      (bind _asbp_mission_control (cast `/Game/Astrumis/Characters/BP_MissionControl` (`Controller.K2_GetPawn` (`GameplayStatics.GetPlayerController` 0))))
      (`/Game/Astrumis/Characters/BP_MissionControl.ServerEndInteract` _asbp_mission_control _interaction_component))))

(fn `PlaySound`
  (locals (DelayTime :type "Float (double-precision)") (Sound :type "SoundBase Object Reference"))
  (bind _audio (`self.Audio`))
  (`|ExecutionSequence`
    (:`then_0`
      (switch `/Game/Astrumis/Doodads/E_DoorState` (`self.State`)
        (:`NewEnumerator2`
          (set `local.DelayTime` (* (`KismetMathLibrary.Abs` (- (`self.ClosingDelta`) 1.0)) (`self.TimeToOpen`)))
          (set `local.Sound` "/Game/Astrumis/Sounds/Interactions/CUE_DoorOpen.CUE_DoorOpen"))
        (:`NewEnumerator3`
          (set `local.DelayTime` (* (`self.ClosingDelta`) (`self.TimeToClose`)))
          (set `local.Sound` "/Game/Astrumis/Sounds/Interactions/CUE_DoorClose.CUE_DoorClose"))))
    (:`then_1`
      (`AudioComponent.Stop` _audio)
      (`AudioComponent.SetSound` _audio (`local.Sound`))
      (`AudioComponent.Play` _audio (`local.DelayTime`)))))

(fn `UserConstructionScript`
  (`parent.UserConstructionScript`))
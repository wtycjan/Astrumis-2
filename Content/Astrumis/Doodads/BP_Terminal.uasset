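; BP_Terminal is an interactable terminal doodad that plays dialogue and advances quests when used.
; Its interactable component's OnInteract event calls InteractWithTerminal, which plays the optional voiceline through the subtitles subsystem for the first player controller.
; It then tries to complete each quest in QuestsToComplete through the quest subsystem.
; When OneTimeUse is set, it clears the component's interacting player type to None after use.
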(event `self.BP_InteractableComponent.OnInteract`
  (params (InteractionIndex :type Integer) (Interactor :type "Actor Object Reference"))
  ;[1 1 1] Interact / End Interact
  (`self.InteractWithTerminal` Interactor))

(event `InteractWithTerminal`
  (params (Interactor :type "Actor Object Reference"))
  (bind _voicelineonpickup (`self.VoicelineOnPickup`))
  ;[1 1 1] Pickup Keycard
  (`/Engine/EditorBlueprintResources/StandardMacros.IsValid` _voicelineonpickup
    (:`Is Valid`
      (`SubtitlesSubsystem.PlayDialogue` (subsystem `/Game/Astrumis/Subtitles/BP_SubtitlesSubsystem`) _voicelineonpickup (`GameplayStatics.GetPlayerController` 0)))
    (:`Is Not Valid`
      _))
  (for _array_element (`self.QuestsToComplete`)
    (`QuestSubsystem.TryCompleteQuest` (subsystem `/Game/Astrumis/Quests/BP_QuestSubsystem`) _array_element))
  (if (`self.bOneTimeUse`)
    (set `/Game/FPFM/Core/Components/FPFM_InteractionComponent.InteractingPlayerType` "None" (`self.BP_InteractableComponent`))))

(fn `UserConstructionScript`
  (`parent.UserConstructionScript`))
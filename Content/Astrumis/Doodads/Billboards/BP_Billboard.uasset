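; BP_Billboard is a doodad that shows or hides its billboard by player proximity, optionally tied to an interactable object.
; Overlaps show it on entering SphereAppear or leaving SphereDissapear, and hide it on the reverse.
; SetBillboardActive's true value means hidden; a linked BP_InteractableComponent forces hiding unless its interacting player type is Survivor or Both.
; BeginPlay caches that component on authority and destroys remote copies.
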(event `self.ReceiveBeginPlay`
  (bind _interactableobject (`self.InteractableObject`))
  (bind _returnvalue (`self.GetComponentByClass` _interactableobject "/Game/Astrumis/Core/BP_InteractableComponent.BP_InteractableComponent_C"))
  ;[0.1306 1 0] BeginPlay
  (`/Engine/EditorBlueprintResources/ActorMacros.Switch Has Authority`
    (:`Authority`
      (`/Engine/EditorBlueprintResources/StandardMacros.IsValid` _interactableobject
        (:`Is Valid`
          (`/Engine/EditorBlueprintResources/StandardMacros.IsValid` _returnvalue
            (:`Is Valid`
              (set `self.InteractableComponent` _returnvalue))))))
    (:`Remote`
      (`self.K2_DestroyActor`))))

(event `self.SphereDissapear.OnComponentBeginOverlap`
  (params (OverlappedComponent :type "PrimitiveComponent Object Reference") (OtherActor :type "Actor Object Reference") (OtherComp :type "PrimitiveComponent Object Reference") (OtherBodyIndex :type Integer) (bFromSweep :type Boolean) (SweepResult :type "HitResult Structure (by ref)"))
  ;[1 1 1] Hide/Show
  (cast `/Game/Astrumis/Characters/BP_AstrumisPlayerCharacter` OtherActor)
  (`self.SetBillboardActive` true))

(event `self.SphereDissapear.OnComponentEndOverlap`
  (params (OverlappedComponent :type "PrimitiveComponent Object Reference") (OtherActor :type "Actor Object Reference") (OtherComp :type "PrimitiveComponent Object Reference") (OtherBodyIndex :type Integer))
  ;[1 1 1] Hide/Show
  (cast `/Game/Astrumis/Characters/BP_AstrumisPlayerCharacter` OtherActor)
  (`self.SetBillboardActive` false))

(event `self.SphereAppear.OnComponentBeginOverlap`
  (params (OverlappedComponent :type "PrimitiveComponent Object Reference") (OtherActor :type "Actor Object Reference") (OtherComp :type "PrimitiveComponent Object Reference") (OtherBodyIndex :type Integer) (bFromSweep :type Boolean) (SweepResult :type "HitResult Structure (by ref)"))
  ;[1 1 1] Hide/Show
  (cast `/Game/Astrumis/Characters/BP_AstrumisPlayerCharacter` OtherActor)
  (`self.SetBillboardActive` false))

(event `self.SphereAppear.OnComponentEndOverlap`
  (params (OverlappedComponent :type "PrimitiveComponent Object Reference") (OtherActor :type "Actor Object Reference") (OtherComp :type "PrimitiveComponent Object Reference") (OtherBodyIndex :type Integer))
  ;[1 1 1] Hide/Show
  (cast `/Game/Astrumis/Characters/BP_AstrumisPlayerCharacter` OtherActor)
  (`self.SetBillboardActive` true))

(fn `SetBillboardActive`
  (params (bValue :type Boolean))
  (bind _billboard (`self.Billboard`))
  (bind _bvalue (`local.bValue`))
  (bind _interactablecomponent (`self.InteractableComponent`))
  (`/Engine/EditorBlueprintResources/StandardMacros.IsValid` _interactablecomponent
    (:`Is Valid`
      (`SceneComponent.SetHiddenInGame` _billboard (select `EInteractingPlayers` (`/Game/FPFM/Core/Components/FPFM_InteractionComponent.InteractingPlayerType` _interactablecomponent) :`None` true :`MissionControl` true :`Survivor` _bvalue :`Both` _bvalue) false))
    (:`Is Not Valid`
      (`SceneComponent.SetHiddenInGame` _billboard (`local.bValue`) false))))

(fn `UserConstructionScript`)
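; Actor component that links a minigame to its in-world consequences through the Guitar Hero subsystem.
; StartMinigame stores the interactor and its location, then binds to the subsystem's success and fail events.
; Each outcome triggers its list of interactables, fires a matching dispatcher and clears the bindings, with success also deactivating the component.
; Failure can raise an alarm that plays a sound and repeatedly reports AI noise at the interactor's stored location.
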(event `Alarm`
  (`GameplayStatics.PlaySoundAtLocation` "/Game/Astrumis/Sounds/Minigames/CUE_AlarmMinigame.CUE_AlarmMinigame" (`Actor.K2_GetActorLocation` (`self.GetOwner`)) (struct) 1.0 1.0 0.0 null null null null)
  (`AISense_Hearing.ReportNoiseEvent` (`self.InteractorLocation`) 1.0 (`self.GetOwner`) 2000.0 "Noise")
  (`KismetSystemLibrary.Delay` 0.4)
  (`AISense_Hearing.ReportNoiseEvent` (`self.InteractorLocation`) 1.0 (`self.GetOwner`) 2000.0 "Noise")
  (`KismetSystemLibrary.Delay` 0.4)
  (`AISense_Hearing.ReportNoiseEvent` (`self.InteractorLocation`) 1.0 (`self.GetOwner`) 2000.0 "Noise")
  (`KismetSystemLibrary.Delay` 0.4)
  (`AISense_Hearing.ReportNoiseEvent` (`self.InteractorLocation`) 1.0 (`self.GetOwner`) 2000.0 "Noise")
  (`KismetSystemLibrary.Delay` 0.4)
  (`AISense_Hearing.ReportNoiseEvent` (`self.InteractorLocation`) 1.0 (`self.GetOwner`) 2000.0 "Noise")
  (`KismetSystemLibrary.Delay` 0.4)
  (`AISense_Hearing.ReportNoiseEvent` (`self.InteractorLocation`) 1.0 (`self.GetOwner`) 2000.0 "Noise"))

(fn `Fail`
  (bind _returnvalue (subsystem `/Game/Astrumis/Minigames/GuitarHero/BP_GuitarHeroSubsystem`))
  (for _array_element (`self.InteractablesOnFail`)
    (`/Game/FPFM/Core/Components/FPFM_InteractionComponent.Interact` (`Actor.GetComponentByClass` _array_element "/Game/Astrumis/Core/BP_InteractableComponent.BP_InteractableComponent_C") 0 (`self.Interactor`)))
  (`self.OnFail`)
  (clear `/Game/Astrumis/Minigames/GuitarHero/BP_GuitarHeroSubsystem.OnFail` _returnvalue)
  (clear `/Game/Astrumis/Minigames/GuitarHero/BP_GuitarHeroSubsystem.OnSuccess` _returnvalue)
  (if (`self.bAlarmOnFail`)
    (`self.Alarm`)))

(fn `StartMinigame`
  (params (Interactor :type "Actor Object Reference"))
  (bind _returnvalue (subsystem `/Game/Astrumis/Minigames/GuitarHero/BP_GuitarHeroSubsystem`))
  (bind _output_get (set `self.Interactor` Interactor))
  (set `self.InteractorLocation` (`Actor.K2_GetActorLocation` _output_get))
  (add `/Game/Astrumis/Minigames/GuitarHero/BP_GuitarHeroSubsystem.OnSuccess` _returnvalue (`|CreateDelegate` :!event `Success`))
  (add `/Game/Astrumis/Minigames/GuitarHero/BP_GuitarHeroSubsystem.OnFail` _returnvalue (`|CreateDelegate` :!event `Fail`)))

(fn `Success`
  (bind _returnvalue (subsystem `/Game/Astrumis/Minigames/GuitarHero/BP_GuitarHeroSubsystem`))
  (`self.Deactivate`)
  (for _array_element (`self.InteractablesOnSuccess`)
    (`/Game/FPFM/Core/Components/FPFM_InteractionComponent.Interact` (`Actor.GetComponentByClass` _array_element "/Game/Astrumis/Core/BP_InteractableComponent.BP_InteractableComponent_C") 0 (`self.Interactor`)))
  (`self.OnSuccess`)
  (clear `/Game/Astrumis/Minigames/GuitarHero/BP_GuitarHeroSubsystem.OnFail` _returnvalue)
  (clear `/Game/Astrumis/Minigames/GuitarHero/BP_GuitarHeroSubsystem.OnSuccess` _returnvalue))
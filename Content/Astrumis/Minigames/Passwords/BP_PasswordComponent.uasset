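; Password component for the Astrumis password minigame that holds a password and a locked state for a lockable object.
; On BeginPlay it generates a password if none is set, padding PasswordKey with random uppercase letters, lowercase letters or digits.
; Each candidate character is re-rolled until it is not already in the password.
; Toggling the lock calls the Unlock dispatcher whenever the state becomes unlocked.
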(event `self.ReceiveBeginPlay`
  (if (`KismetStringLibrary.IsEmpty` (`self.Password`))
    (`self.CreatePassword`)))

(event `ToggleLockedStatus`
  (bind _output_get (set `self.bLocked` (not (`self.bLocked`))))
  (if (not _output_get)
    (`self.Unlock`)))

(fn `CreatePassword`
  (locals (TempPassword :type String) (NewCharacter :type String))
  (bind _passwordkey (`self.PasswordKey`))
  (bind _outitem (`KismetArrayLibrary.Array_Random` (`self.Alphabet`)))
  (set `local.TempPassword` _passwordkey)
  (for _ (range (`KismetStringLibrary.Len` _passwordkey) 7)
    (switch `int` (`KismetMathLibrary.RandomIntegerInRange` 0 2)
      (:`0`
        (bind _output_get (set `local.NewCharacter` _outitem :!label _label))
        (if (`KismetStringLibrary.Contains` (`local.TempPassword`) _output_get)
          (goto _label)
          (else
            (set `local.NewCharacter` (`KismetStringLibrary.ToUpper` (`local.NewCharacter`))))))
      (:`1`
        (bind _output_get_2 (set `local.NewCharacter` _outitem :!label _label_2))
        (if (`KismetStringLibrary.Contains` (`local.TempPassword`) _output_get_2)
          (goto _label_2)
          (else
            (set `local.NewCharacter` (`KismetStringLibrary.ToLower` (`local.NewCharacter`))))))
      (:`2`
        (bind _output_get_3 (set `local.NewCharacter` (`KismetStringLibrary.Conv_IntToString` (`KismetMathLibrary.RandomIntegerInRange` 0 9)) :!label _label_3))
        (if (`KismetStringLibrary.Contains` (`local.TempPassword`) _output_get_3)
          (goto _label_3)
          (else
            _))))
    (set `local.TempPassword` (`KismetStringLibrary.Concat_StrStr` (`local.TempPassword`) (`local.NewCharacter`))))
  (set `self.Password` (`local.TempPassword`)))
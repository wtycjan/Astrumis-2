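; Anim notify that plays the monster's footstep sound at the left or right foot socket, chosen by its LeftFoot flag.
; It calls GetSurface on ABP_Monster and picks a cue through a surface-type Select, playing it only if valid.
; Only the Default surface has a cue; Grass, Dirt, Rock and Wood are empty.
; An unconnected selection keyed on the blackboard's player-detected flag remains unused.
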(fn `Received_Notify`
  (params (MeshComp :type "SkeletalMeshComponent Object Reference") (Animation :type "AnimSequenceBase Object Reference") (EventReference :type "AnimNotifyEventReference Structure (by ref)"))
  (returns (ReturnValue :type Boolean))
  (locals (Mesh :type "SkeletalMeshComponent Object Reference") (CurrentPlayerGait :type "/Game/FPFM/Core/Enums/E_GaitTypes Enum"))
  (bind _returnvalue (select `EPhysicalSurface` "SurfaceType_Default" :`SurfaceType_Default` "/Game/Astrumis/Sounds/Footsteps/MonsterWalkFootstep/CUE_MonsterWalkFootstep.CUE_MonsterWalkFootstep" :!type "SoundBase Object Reference"))
  (bind _leftfoot_ (`self.LeftFoot?`))
  ;[0 0 0] Play Footstep sound at foot location
  (`/Engine/EditorBlueprintResources/StandardMacros.IsValid` MeshComp
    (:`Is Valid`
      (bind _output_get (set `local.Mesh` MeshComp))
      (`/Game/Astrumis/Animations/Monster/ABP_Monster.GetSurface` (cast `/Game/Astrumis/Animations/Monster/ABP_Monster` (`SkeletalMeshComponent.GetAnimInstance` (`local.Mesh`)) :!pure true) _leftfoot_)
      (`/Engine/EditorBlueprintResources/StandardMacros.IsValid` _returnvalue
        (:`Is Valid`
          (`GameplayStatics.PlaySoundAtLocation` _returnvalue (`SceneComponent.GetSocketLocation` (`local.Mesh`) (select `bool` _leftfoot_ :`false` "foot_r" :`true` "foot_l" :!type "Name")) (struct) 1.0 1.0 0.0 null null null null)
          (return false))))))
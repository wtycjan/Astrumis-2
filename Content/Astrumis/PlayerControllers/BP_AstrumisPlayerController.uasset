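; BP_AstrumisPlayerController is the Astrumis player controller that owns and opens the pause menu.
; On BeginPlay it creates WBP_PauseMenuAstrumis once, adds it to the viewport and keeps a reference.
; Escape or Divide switches to UI-only input, shows the mouse cursor and makes the menu visible through TogglePauseMenu.
; Nothing here pauses the game, restores game input or calls for the menu to hide.
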(event `self.ReceiveBeginPlay`
  (`self.CreatePauseMenu`))

(event `Key|Escape`
  (params (Key :type "Key Structure"))
  (:`Pressed`
    (`WidgetBlueprintLibrary.SetInputMode_UIOnlyEx` self null :!label _label)
    (set `self.bShowMouseCursor` true)
    (`self.TogglePauseMenu` true)))

(event `Key|Divide`
  (params (Key :type "Key Structure"))
  (:`Pressed`
    (goto _label)))

(event `CreatePauseMenu`
  ;[1 1 1] Pause Menu
  (bind _returnvalue (`|CreateWidget` "/Game/Astrumis/Core/UI/WBP_PauseMenuAstrumis.WBP_PauseMenuAstrumis_C" self))
  (bind _output_get (set `self.WBP_PauseMenu` _returnvalue))
  (`UserWidget.AddToViewport` _output_get 0))

(event `TogglePauseMenu`
  (params (bVisible :type Boolean))
  ;[1 1 1] Pause Menu
  (`Widget.SetVisibility` (`self.WBP_PauseMenu`) (select `bool` bVisible :`false` "Hidden" :`true` "Visible" :!type "ESlateVisibility Enum")))

(fn `UserConstructionScript`
  (`parent.UserConstructionScript`))